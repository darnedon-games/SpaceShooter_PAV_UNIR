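; BP_EnemyHorizontal is an enemy variant that sets a sideways movement vector and reverses it at lateral boundaries.
; It starts along its right vector and flips direction whenever it overlaps an actor tagged "Lateral".
; Each right-to-left flip also shortens DelayShoot, with no lower limit here.
; Move only calls the parent implementation, and the Tick override is disabled.
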(event EventBeginPlay
  (|CallParentFunction)
  (Variables|Default|SetMovementVector (Transformation|GetActorRightVector))
  (Variables|Default|SetIsRight true))

(event Collision|EventActorBeginOverlap
  (params (OtherActor :type Actor%20Object%20Reference))
  (bind _returnvalue (Transformation|GetActorRightVector))
  (|CallParentFunction OtherActor)
  (if (Utilities|Array|ContainsItem (Variables|/Script/Engine.Actor|GetTags OtherActor) "Lateral")
    (if (Variables|Default|GetIsRight)
      (Variables|Default|SetIsRight false)
      (Variables|Default|SetMovementVector (* _returnvalue "-1.0,-1.0,-1.0"))
      (Variables|Default|SetDelayShoot (- (Variables|Default|GetDelayShoot) 0.1))
      (else
        (Variables|Default|SetIsRight true)
        (Variables|Default|SetMovementVector _returnvalue)))))

(event EventTick
  (params (DeltaSeconds :type Float%20%28single-precision%29))
  (|CallParentFunction DeltaSeconds) ; This node is disabled and will not be called.\nDrag off pins to build functionality.
)

(fn ConstructionScript
  (|CallParentFunction))

(fn Move
  (params (DeltaTime :type Float%20%28double-precision%29))
  (|CallParentFunction DeltaTime))