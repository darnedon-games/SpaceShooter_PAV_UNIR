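; BP_ObjectsGenerator is a spawner actor that periodically creates BP_SS_Lives actors in the game.
; BeginPlay starts a looping timer at the SpawnTime interval, which fires the Spawn event and calls SpawnObject.
; SpawnObject picks a random scene component tagged "SpawnPoint" on itself, spawns the actor at that component's world transform and returns it.
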(event Custom|Spawn
  (CallFunction|SpawnObject))

(event EventBeginPlay
  (Utilities|Time|SetTimerbyEvent (delegate Custom|Spawn) (Variables|Default|GetSpawnTime) true))

(event Collision|EventActorBeginOverlap
  (params (OtherActor :type Actor%20Object%20Reference)))

(event EventTick
  (params (DeltaSeconds :type Float%20%28single-precision%29)))

(fn ConstructionScript)

(fn SpawnObject
  (bind _returnvalue (Actor|GetComponentsbyTag "/Script/Engine.SceneComponent" "SpawnPoint"))
  (bind _returnvalue_2 (Game|SpawnActorfromClass "/Game/Players/BP_SS_Lives.BP_SS_Lives_C" (Transformation|GetWorldTransform (Utilities|Array|Get(acopy) _returnvalue (Math|Random|RandomInteger (Utilities|Array|Length _returnvalue)))) "Undefined" "MultiplyWithRoot" 0 0))
  (return _returnvalue_2))