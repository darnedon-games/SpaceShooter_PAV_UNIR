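; BP_SpaceSPlayer is the player-controlled pawn, which moves and fires bullets.
; On BeginPlay it registers the BP_InputMapping Enhanced Input context with its player controller.
; The move action feeds movement input along the actor's right and forward vectors.
; The fire action spawns a Bullet at BulletPoint through DoFire, rate-limited by a CanFire flag that a timer resets after FireDelay.
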(event Custom|UpdateFire
  (Variables|Default|SetCanFire true))

(event Input|EnhancedActionEvents|EnhancedInputActionBP_InputMove
  (params (ActionValue :type Vector%202D%20Structure) (ElapsedSeconds :type Float%20%28double-precision%29) (TriggeredSeconds :type Float%20%28double-precision%29) (InputAction :type Input%20Action%20Object%20Reference :default "/Game/Input/BP_InputMove.BP_InputMove"))
  (:Triggered
    (Pawn|Input|AddMovementInput (Transformation|GetActorRightVector) (.x ActionValue) false)
    (Pawn|Input|AddMovementInput (Transformation|GetActorForwardVector) (.y ActionValue) false)))

(event Input|EnhancedActionEvents|EnhancedInputActionBP_InputFire
  (params (ActionValue :type Boolean) (ElapsedSeconds :type Float%20%28double-precision%29) (TriggeredSeconds :type Float%20%28double-precision%29) (InputAction :type Input%20Action%20Object%20Reference :default "/Game/Input/BP_InputFire.BP_InputFire"))
  (:Triggered
    (if (Variables|Default|GetCanFire)
      (CallFunction|DoFire)
      (Variables|Default|SetCanFire false)
      (Utilities|Time|SetTimerbyEvent (delegate Custom|UpdateFire) (Variables|Default|GetFireDelay)))))

(event EventBeginPlay
  ;[1 1 1] Comprobar que el puntero no sea nulo
  (bind _asplayer_controller (Utilities|Casting|CastToPlayerController (Pawn|GetController)))
  (Utilities|IsValid (PlayerController|LocalPlayerSubsystems|GetEnhancedInputLocalPlayerSubsystem _asplayer_controller)
    (:Is%20Valid
      (Input|AddMappingContext (PlayerController|LocalPlayerSubsystems|GetEnhancedInputLocalPlayerSubsystem _asplayer_controller) "/Game/Input/BP_InputMapping.BP_InputMapping" 0 "(bIgnoreAllPressedKeysUntilRelease=True,bForceImmediately=False,bNotifyUserSettings=False)"))))

(event Collision|EventActorBeginOverlap
  (params (OtherActor :type Actor%20Object%20Reference)))

(event EventTick
  (params (DeltaSeconds :type Float%20%28single-precision%29)))

(fn ConstructionScript)

(fn DoFire
  (Game|SpawnActorfromClass (Variables|Default|GetBullet) (Transformation|GetWorldTransform (Variables|Default|GetBulletPoint)) "Undefined" "MultiplyWithRoot" 0 0))